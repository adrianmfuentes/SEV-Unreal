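; Ranged enemy that wanders to random reachable points and shoots the player, using a weapon it spawns on its mesh socket.
; PawnSensing sightings turn it toward the player and fire, with a retriggerable delay restarting the wander once sightings pause.
; Tick updates the health bar widget and yaws it toward the player.
; Each hit removes fixed health; death awards the player a point and destroys the first attached actor and itself.
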(event `self.ReceiveBeginPlay`
  (`self.Configure weapon`)
  (bind _asbp_player (cast `/Game/Player/Blueprints/BP_Player` (`GameplayStatics.GetPlayerCharacter` 0)))
  (set `self.JugadorReferencia` _asbp_player)
  (`self.GoToRandomPoint`))

(event `GoToRandomPoint`
  (`|AIMoveTo` self (`NavigationSystemV1.K2_GetRandomReachablePointInRadius` (`self.K2_GetActorLocation`) 2500.0 null null) null
    (:`OnSuccess`
      (`self.GoToRandomPoint`))))

(event `self.PawnSensing.OnSeePawn`
  (params (Pawn :type "Pawn Object Reference"))
  (`|ExecutionSequence`
    (:`then_0`
      (`self.K2_SetActorRotation` (`KismetMathLibrary.FindLookAtRotation` (`self.K2_GetActorLocation`) (`self.K2_GetActorLocation` (`self.JugadorReferencia`))))
      (`/Game/IA-Enemigo/Enemigo_Dispara/Enemigo3Weapon.Shoot` (`self.weapon`)))
    (:`then_1`
      (`KismetSystemLibrary.RetriggerableDelay` 0.8)
      (`self.GoToRandomPoint`))))

(event `Configure weapon`
  (bind _returnvalue (`|SpawnActorFromClass` "/Game/IA-Enemigo/Enemigo_Dispara/Enemigo3Weapon.Enemigo3Weapon_C" (`KismetMathLibrary.Conv_VectorToTransform` (`SceneComponent.K2_GetComponentLocation` (`self.Sphere`))) "Undefined" "OverrideRootScale" null null))
  (bind _output_get (set `self.weapon` _returnvalue))
  (`self.K2_AttachToComponent` _output_get (`self.Mesh`) "weaponSocket" "SnapToTarget" "SnapToTarget" "SnapToTarget" true))

(event `self.ReceiveTick`
  (params (DeltaSeconds :type "Float (single-precision)"))
  (bind (_returnvalue_roll _returnvalue_pitch _returnvalue_yaw) (`KismetMathLibrary.BreakRotator` (`KismetMathLibrary.FindLookAtRotation` (`SceneComponent.K2_GetComponentLocation` (`self.Salud`)) (`self.K2_GetActorLocation` (`self.JugadorReferencia`)))))
  (bind _asvida_enemigo (cast `/Game/IA-Enemigo/vida_enemigo` (`WidgetComponent.GetUserWidgetObject` (`self.Salud`))))
  (`ProgressBar.SetPercent` (`/Game/IA-Enemigo/vida_enemigo.Barra_vida` _asvida_enemigo) (/ (`self.vida`) 150.0))
  (`SceneComponent.K2_SetWorldRotation` (`self.Salud`) (`KismetMathLibrary.MakeRotator` 0.0 0.0 _returnvalue_yaw) false false))

(event `RecibirDaño`
  (set `self.Vida` (- (`self.Vida`) 20.0))
  (if (<= (`self.Vida`) 0.0)
    (set `self.Dying` true)
    (bind _asbp_player (cast `/Game/Player/Blueprints/BP_Player` (`GameplayStatics.GetPlayerCharacter` 0)))
    (`/Engine/EditorBlueprintResources/StandardMacros.IncrementFloat` (`/Game/Player/Blueprints/BP_Player.Puntos` _asbp_player)
      (:`  `
        (`self.K2_DestroyActor` (`|GetArrayItem` (`self.GetAttachedActors` true)))
        (`self.K2_DestroyActor`)))))

(fn `UserConstructionScript`)