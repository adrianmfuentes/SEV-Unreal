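; Enemy pawn that wanders and flees from the player when it sees a pawn, with health and a floating health bar.
; It loops random reachable moves until PawnSensing fires, then speeds up and repeatedly runs directly away from the player.
; A retriggerable delay restores slow wandering once sightings stop.
; Tick updates the widget bar and turns it toward the player; lethal damage adds a player point and destroys the enemy.
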(event `self.ReceiveBeginPlay`
  (bind _asbp_player (cast `/Game/Player/Blueprints/BP_Player` (`GameplayStatics.GetPlayerCharacter` 0)))
  (set `self.JugadorReferencia` _asbp_player)
  (`self.GoToRandomPoint`))

(event `Huir`
  (bind _returnvalue (`self.K2_GetActorLocation`))
  (`|AIMoveTo` self (`KismetMathLibrary.MakeVector` (.x (+ _returnvalue (* (`KismetMathLibrary.GetForwardVector` (`KismetMathLibrary.FindLookAtRotation` _returnvalue (`self.K2_GetActorLocation` (`self.JugadorReferencia`)))) -500.0))) (.y (+ _returnvalue (* (`KismetMathLibrary.GetForwardVector` (`KismetMathLibrary.FindLookAtRotation` _returnvalue (`self.K2_GetActorLocation` (`self.JugadorReferencia`)))) -500.0))) (.z _returnvalue)) null
    (:`OnSuccess`
      _)
    (:`OnFail`
      _))
  (`self.Huir`))

(event `GoToRandomPoint`
  (`|AIMoveTo` self (`NavigationSystemV1.K2_GetRandomReachablePointInRadius` (`self.K2_GetActorLocation`) 2500.0 null null) null
    (:`OnSuccess`
      (`self.GoToRandomPoint`))))

(event `self.PawnSensing.OnSeePawn`
  (params (Pawn :type "Pawn Object Reference"))
  (`|ExecutionSequence`
    (:`then_0`
      (set `CharacterMovementComponent.MaxWalkSpeed` 600.0 (`self.CharacterMovement`))
      (`self.Huir`))
    (:`then_1`
      (`KismetSystemLibrary.RetriggerableDelay` 0.8)
      (set `CharacterMovementComponent.MaxWalkSpeed` 200.0 (`self.CharacterMovement`))
      (`self.GoToRandomPoint`))))

(event `self.ReceiveTick`
  (params (DeltaSeconds :type "Float (single-precision)"))
  (bind (_returnvalue_roll _returnvalue_pitch _returnvalue_yaw) (`KismetMathLibrary.BreakRotator` (`KismetMathLibrary.FindLookAtRotation` (`SceneComponent.K2_GetComponentLocation` (`self.Salud`)) (`self.K2_GetActorLocation` (`self.JugadorReferencia`)))))
  (bind _asvida_enemigo (cast `/Game/IA-Enemigo/vida_enemigo` (`WidgetComponent.GetUserWidgetObject` (`self.Salud`))))
  (`ProgressBar.SetPercent` (`/Game/IA-Enemigo/vida_enemigo.Barra_vida` _asvida_enemigo) (/ (`self.vida`) 50.0))
  (`SceneComponent.K2_SetWorldRotation` (`self.Salud`) (`KismetMathLibrary.MakeRotator` 0.0 0.0 _returnvalue_yaw) false false))

(event `RecibirDaño`
  (set `self.Vida` (- (`self.Vida`) 20.0))
  (if (<= (`self.Vida`) 0.0)
    (set `self.Dying` true)
    (bind _asbp_player (cast `/Game/Player/Blueprints/BP_Player` (`GameplayStatics.GetPlayerCharacter` 0)))
    (`/Engine/EditorBlueprintResources/StandardMacros.IncrementFloat` (`/Game/Player/Blueprints/BP_Player.Puntos` _asbp_player)
      (:`  `
        (`self.K2_DestroyActor`)))))

(fn `UserConstructionScript`)