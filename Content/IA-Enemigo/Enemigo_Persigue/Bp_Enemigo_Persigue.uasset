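; Enemy AI that wanders between random reachable points, chases the player on sight and attacks in melee.
; PawnSensing triggers a faster chase, attacking within range unless the shield is active; a retriggerable delay resumes slow wandering when sightings stop.
; Damage lowers health, and death awards the player a point.
; Tick updates the health bar, turns it toward the player and re-caches the player reference, overriding the sphere overlap's clearing.
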(event `self.ReceiveBeginPlay`
  (bind _asbp_player (cast `/Game/Player/Blueprints/BP_Player` (`GameplayStatics.GetPlayerCharacter` 0)))
  (set `self.JugadorReferencia ` _asbp_player)
  (`self.GoToRandomPoint`))

(event `GoToRandomPoint`
  (`|AIMoveTo` self (`NavigationSystemV1.K2_GetRandomReachablePointInRadius` (`self.K2_GetActorLocation`) 2500.0 null null) null
    (:`OnSuccess`
      (`self.GoToRandomPoint`))))

(event `self.PawnSensing.OnSeePawn`
  (params (Pawn :type "Pawn Object Reference"))
  (`|ExecutionSequence`
    (:`then_0`
      (set `CharacterMovementComponent.MaxWalkSpeed` 600.0 (`self.CharacterMovement`))
      (`|AIMoveTo` self (0.0 0.0 0.0) (`GameplayStatics.GetPlayerPawn` 0)
        (:`OnSuccess`
          (if (<= (`self.GetDistanceTo` (`GameplayStatics.GetPlayerPawn` 0)) (`self.DistanciaDeAtaque `))
            (if (not (`/Game/Player/Blueprints/BP_Player.escudoActivo` (`self.JugadorReferencia `)))
              (`self.Atacar`))))))
    (:`then_1`
      (`KismetSystemLibrary.RetriggerableDelay` 0.8)
      (set `CharacterMovementComponent.MaxWalkSpeed` 200.0 (`self.CharacterMovement`))
      (`self.GoToRandomPoint`))))

(event `self.Sphere.OnComponentBeginOverlap`
  (params (OverlappedComponent :type "PrimitiveComponent Object Reference") (OtherActor :type "Actor Object Reference") (OtherComp :type "PrimitiveComponent Object Reference") (OtherBodyIndex :type Integer) (bFromSweep :type Boolean) (SweepResult :type "HitResult Structure (by ref)"))
  (bind _asbp_player (cast `/Game/Player/Blueprints/BP_Player` OtherActor))
  (set `self.JugadorReferencia ` _asbp_player))

(event `self.Sphere.OnComponentEndOverlap`
  (params (OverlappedComponent :type "PrimitiveComponent Object Reference") (OtherActor :type "Actor Object Reference") (OtherComp :type "PrimitiveComponent Object Reference") (OtherBodyIndex :type Integer))
  (cast `/Game/Player/Blueprints/BP_Player` OtherActor)
  (set `self.JugadorReferencia ` null))

(event `Atacar`
  (if (`KismetSystemLibrary.IsValid` (`self.JugadorReferencia `))
    (set `self.Anim Is Attacking` true)
    (`KismetSystemLibrary.Delay` 0.2)
    (if (`KismetSystemLibrary.IsValid` (`self.JugadorReferencia `))
      (`/Game/Player/Blueprints/BP_Player.RecibirDaño` (`self.JugadorReferencia `))
      (`KismetSystemLibrary.Delay` 0.5)
      (set `self.Anim Is Attacking` false)
      (`KismetSystemLibrary.Delay` 0.2)
      (`GameplayStatics.PlaySound2D` "/Game/Sonidos/ataque_enemigo.ataque_enemigo" 1.0 1.0 0.0 null null))))

(event `RecibirDaño`
  (set `self.Vida` (- (`self.Vida`) 20.0))
  (if (<= (`self.Vida`) 0.0)
    (set `self.Dying` true)
    (bind _asbp_player (cast `/Game/Player/Blueprints/BP_Player` (`GameplayStatics.GetPlayerCharacter` 0)))
    (`/Engine/EditorBlueprintResources/StandardMacros.IncrementFloat` (`/Game/Player/Blueprints/BP_Player.Puntos` _asbp_player)
      (:`  `
        (`self.K2_DestroyActor`)))))

(event `self.ReceiveTick`
  (params (DeltaSeconds :type "Float (single-precision)"))
  (bind (_returnvalue_roll _returnvalue_pitch _returnvalue_yaw) (`KismetMathLibrary.BreakRotator` (`KismetMathLibrary.FindLookAtRotation` (`SceneComponent.K2_GetComponentLocation` (`self.Salud`)) (`self.K2_GetActorLocation` (`self.JugadorReferencia `)))))
  (bind _asbp_player (cast `/Game/Player/Blueprints/BP_Player` (`GameplayStatics.GetPlayerCharacter` 0)))
  (set `self.JugadorReferencia ` _asbp_player)
  (bind _asvida_enemigo (cast `/Game/IA-Enemigo/vida_enemigo` (`WidgetComponent.GetUserWidgetObject` (`self.Salud`))))
  (`ProgressBar.SetPercent` (`/Game/IA-Enemigo/vida_enemigo.Barra_vida` _asvida_enemigo) (/ (`self.vida`) 80.0))
  (`SceneComponent.K2_SetWorldRotation` (`self.Salud`) (`KismetMathLibrary.MakeRotator` 0.0 0.0 _returnvalue_yaw) false false))

(fn `UserConstructionScript`)