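; BP_Linterna is the player's flashlight, which doubles as an automatic laser-style weapon.
; PressTrigger fires at once and starts a looping timer for repeat shots, which ReleaseTrigger clears.
; Each shot spawns a Bp_Linterna_proyectil at the ShootingPoint transform and plays a 2D laser sound.
; A separate ON/OFF event toggles the SpotLight, and BeginPlay caches a BP_Player reference.
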(event `Press Trigger`
  (bind _returnvalue (`KismetSystemLibrary.K2_SetTimer` null "shoot" 0.2 true))
  (`self.Shoot`))

(event `ReleaseTrigger`
  (`KismetSystemLibrary.K2_ClearAndInvalidateTimerHandle` (stale `Press Trigger` _returnvalue)))

(event `self.ReceiveBeginPlay`
  (bind _asbp_player (cast `/Game/Player/Blueprints/BP_Player` (`GameplayStatics.GetPlayerCharacter` 0)))
  (set `self.playerRef` _asbp_player))

(event `Shoot`
  (`|SpawnActorFromClass` "/Game/Player/Linterna/Bp_Linterna_proyectil.Bp_Linterna_proyectil_C" (`SceneComponent.K2_GetComponentToWorld` (`self.ShootingPoint`)) "Undefined" "OverrideRootScale" null null)
  (`GameplayStatics.PlaySound2D` "/Game/Sonidos/laser.laser" 1.0 1.0 0.0 null null))

(event `ON/OFF`
  (`SceneComponent.ToggleVisibility` (`self.SpotLight`) false))

(fn `UserConstructionScript`)