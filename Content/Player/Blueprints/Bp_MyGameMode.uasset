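; Game mode that runs a level's HUD, scoring and progression.
; On BeginPlay it creates and shows the InGameHUDW widget, and a restart event reopens the current level by name.
; Each EnemyDestroyed call adds a point, and at five points a DoOnce increments Level on MyGameInstance and opens the level named after that number.
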(event `self.ReceiveBeginPlay`
  (bind _returnvalue (`|CreateWidget` "/Game/InGameHUDW.InGameHUDW_C"))
  (`UserWidget.AddToViewport` _returnvalue 0))

(event `RestartCurrentLevel`
  (bind _returnvalue (`GameplayStatics.GetCurrentLevelName` true))
  (`GameplayStatics.OpenLevel` (`KismetStringLibrary.Conv_StringToName` _returnvalue)))

(event `EnemyDestroyed`
  (bind _result (`/Engine/EditorBlueprintResources/StandardMacros.IncrementInt` (`self.Points`))
    (:`  `
      (bind _output_get (set `self.Points` _result))
      (`KismetSystemLibrary.PrintString` (`KismetStringLibrary.Conv_IntToString` _output_get))
      (if (>= (`self.Points`) 5)
        (`/Engine/EditorBlueprintResources/StandardMacros.DoOnce` false
          (:`Completed`
            (bind _asmy_game_instance (cast `/Game/MyGameInstance` (`GameplayStatics.GetGameInstance`)))
            (bind _output_get_2 (set `/Game/MyGameInstance.level` (+ (`/Game/MyGameInstance.level` _asmy_game_instance) 1) _asmy_game_instance))
            (`GameplayStatics.OpenLevel` (`KismetStringLibrary.Conv_StringToName` (`KismetStringLibrary.Concat_StrStr` "" (`KismetStringLibrary.Conv_IntToString` _output_get_2))))))))))

(fn `UserConstructionScript`)