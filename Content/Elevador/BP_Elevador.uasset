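; Elevator actor that the player toggles up and down with the IA_Ascensor input while inside its Box trigger.
; Box overlap by BP_Player enables input and opens a Gate; leaving disables and closes them.
; A FlipFlop alternates two MoveComponentTo nodes on the Cube, each stopping the other before moving, so travel can reverse midway.
; Completing the upward trip sets the player's Llave (key) to 0.
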(event `EnhancedInput|/Game/Input/Actions/IA_Ascensor`
  (params (ActionValue :type Boolean) (ElapsedSeconds :type "Float (double-precision)") (TriggeredSeconds :type "Float (double-precision)") (InputAction :type "InputAction Object Reference" :default "/Game/Input/Actions/IA_Ascensor.IA_Ascensor"))
  (bind _cube (`self.Cube`))
  (:`Started`
    (`/Engine/EditorBlueprintResources/StandardMacros.Gate` true :!label _label
      (:`Exit`
        (`/Engine/EditorBlueprintResources/StandardMacros.FlipFlop`
          (:`A`
            (`|ExecutionSequence`
              (:`then_0`
                (goto _label_3 :!via `Stop`))
              (:`then_1`
                (`KismetSystemLibrary.MoveComponentTo` _cube (0.0 0.0 380.0) (struct) false false 2.0 :!label _label_2)
                (bind _asbp_player (cast `/Game/Player/Blueprints/BP_Player` (`GameplayStatics.GetPlayerCharacter` 0)))
                (set `/Game/Player/Blueprints/BP_Player.llave` 0 _asbp_player))))
          (:`B`
            (`|ExecutionSequence`
              (:`then_0`
                (goto _label_2 :!via `Stop`))
              (:`then_1`
                (`KismetSystemLibrary.MoveComponentTo` _cube (0.0 0.0 0.0) (struct) false false 2.0 :!label _label_3)))))))))

(event `self.Box.OnComponentBeginOverlap`
  (params (OverlappedComponent :type "PrimitiveComponent Object Reference") (OtherActor :type "Actor Object Reference") (OtherComp :type "PrimitiveComponent Object Reference") (OtherBodyIndex :type Integer) (bFromSweep :type Boolean) (SweepResult :type "HitResult Structure (by ref)"))
  (cast `/Game/Player/Blueprints/BP_Player` OtherActor)
  (`self.EnableInput` (`GameplayStatics.GetPlayerController` 0))
  (goto _label :!via `Open`))

(event `self.Box.OnComponentEndOverlap`
  (params (OverlappedComponent :type "PrimitiveComponent Object Reference") (OtherActor :type "Actor Object Reference") (OtherComp :type "PrimitiveComponent Object Reference") (OtherBodyIndex :type Integer))
  (cast `/Game/Player/Blueprints/BP_Player` OtherActor)
  (`self.DisableInput` (`GameplayStatics.GetPlayerController` 0))
  (goto _label :!via `Close`))

(fn `UserConstructionScript`)