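; Breakable puzzle crate that a player holding the revolver can smash to drop a key.
; Box overlap enables input on the crate if BP_Player has the revolver, otherwise prints a hint; leaving the box disables it.
; IA_Interact calls RomperCaja, which fires particles and an explosion sound and spawns Bp_Llave through a DoOnce, then the crate destroys itself after a short delay.
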(event `self.Box.OnComponentBeginOverlap`
  (params (OverlappedComponent :type "PrimitiveComponent Object Reference") (OtherActor :type "Actor Object Reference") (OtherComp :type "PrimitiveComponent Object Reference") (OtherBodyIndex :type Integer) (bFromSweep :type Boolean) (SweepResult :type "HitResult Structure (by ref)"))
  (bind _asbp_player (cast `/Game/Player/Blueprints/BP_Player` OtherActor))
  (if (`/Game/Player/Blueprints/BP_Player.hasRevolver` _asbp_player)
    (`self.EnableInput` (`GameplayStatics.GetPlayerController` 0))
    (else
      (`KismetSystemLibrary.PrintString` "Te hace falta algo para romper la caja"))))

(event `self.Box.OnComponentEndOverlap`
  (params (OverlappedComponent :type "PrimitiveComponent Object Reference") (OtherActor :type "Actor Object Reference") (OtherComp :type "PrimitiveComponent Object Reference") (OtherBodyIndex :type Integer))
  (cast `/Game/Player/Blueprints/BP_Player` OtherActor)
  (`self.DisableInput` (`GameplayStatics.GetPlayerController` 0)))

(event `EnhancedInput|/Game/Input/Actions/IA_Interact`
  (params (ActionValue :type Boolean) (ElapsedSeconds :type "Float (double-precision)") (TriggeredSeconds :type "Float (double-precision)") (InputAction :type "InputAction Object Reference" :default "/Game/Input/Actions/IA_Interact.IA_Interact"))
  (:`Triggered`
    (`self.RomperCaja`)
    (`KismetSystemLibrary.Delay` 0.2)
    (`self.K2_DestroyActor`)))

(event `RomperCaja`
  (`ActorComponent.Activate` (`self.ParticleSystem`) false)
  (`GameplayStatics.PlaySound2D` "/Game/StarterContent/Audio/Explosion_Cue.Explosion_Cue" 1.0 1.0 0.0 null null)
  (`/Engine/EditorBlueprintResources/StandardMacros.DoOnce` false
    (:`Completed`
      (`|SpawnActorFromClass` "/Game/Puerta/Bp_Llave.Bp_Llave_C" (`self.GetTransform`) "Undefined" "OverrideRootScale" null null))))

(fn `UserConstructionScript`)