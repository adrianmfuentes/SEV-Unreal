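; Gate actor for a lever puzzle that removes itself once three levers are active.
; Every tick it fetches the first Bp_Palanca, Bp_Palanca1 and Bp_Palanca2 through GetAllActorsOfClass and checks each EstaActivo flag in nested branches.
; When all three are true, it calls DestroyActor, with no animation or other feedback.
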(event `self.ReceiveTick`
  (params (DeltaSeconds :type "Float (single-precision)"))
  (bind _outactors (`GameplayStatics.GetAllActorsOfClass` "/Game/Puzzles/Palancas/Bp_Palanca.Bp_Palanca_C"))
  (if (`/Game/Puzzles/Palancas/Bp_Palanca.EstaActivo` (`|GetArrayItem` _outactors))
    (bind _outactors_2 (`GameplayStatics.GetAllActorsOfClass` "/Game/Puzzles/Palancas/Bp_Palanca1.Bp_Palanca1_C"))
    (if (`/Game/Puzzles/Palancas/Bp_Palanca1.EstaActivo` (`|GetArrayItem` _outactors_2))
      (bind _outactors_3 (`GameplayStatics.GetAllActorsOfClass` "/Game/Puzzles/Palancas/Bp_Palanca2.Bp_Palanca2_C"))
      (if (`/Game/Puzzles/Palancas/Bp_Palanca2.EstaActivo` (`|GetArrayItem` _outactors_3))
        (`self.K2_DestroyActor`)))))

(fn `UserConstructionScript`)